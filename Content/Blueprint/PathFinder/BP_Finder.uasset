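; Pathfinding actor that lays a node grid over the actor tagged "Plain" and offers A*, Dijkstra and BFS through an on-screen UI.
; BeginPlay creates the widget, binds its buttons to algorithm delegates, then finds the area.
; A self-re-entering MultiGate steps through SetMinMaxBound, storing absolute min/max X and Y from the area's bounds with debug prints.
; It then calls DrawGrid and sets the first and last nodes as start and destination.
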(event `self.SetBound`
  (bind _nodearray (`self.NodeArray`))
  (bind (_origin _boxextent) (`self.GetActorBounds` (`self.Area`) false false))
  (set `self.NodeDensity` (`self.NodeDensity`))
  (bind _output_get (set `self.SavedArea` (`self.Area`)))
  (`KismetSystemLibrary.PrintString` (`KismetSystemLibrary.GetDisplayName` _output_get) true true (struct :`G` 0.66 :`B` 1.0 :`A` 1.0) 15.0)
  (`|MultiGate` false :!label _label
    (:`Out 0`
      (bind _output_get_2 (set `self.minX` (`KismetMathLibrary.Abs` (- (.x _origin) (.x _boxextent)))))
      (set `self.CurrentNodePos_X` _output_get_2)
      (set `self.TopZ` 0.0)
      (`KismetSystemLibrary.PrintString` (`KismetStringLibrary.Concat_StrStr` "Current  X :" (`KismetStringLibrary.Conv_DoubleToString` _output_get_2)) true true (struct :`G` 0.66 :`B` 1.0 :`A` 1.0) 11.0)
      (goto _label))
    (:`Out 1`
      (bind _output_get_3 (set `self.MinY` (`KismetMathLibrary.Abs` (- (.y _origin) (.y _boxextent)))))
      (set `self.CurrentNodePos_Y` _output_get_3)
      (`KismetSystemLibrary.PrintString` (`KismetStringLibrary.Concat_StrStr` "Current Y :" (`KismetStringLibrary.Conv_DoubleToString` _output_get_3)) true true (struct :`G` 0.66 :`B` 1.0 :`A` 1.0) 11.0)
      (goto _label))
    (:`Out 2`
      (bind _output_get_4 (set `self.MaxX` (`KismetMathLibrary.Abs` (+ (.x _origin) (.x _boxextent)))))
      (set `self.MaxArea_X` _output_get_4)
      (`KismetSystemLibrary.PrintString` (`KismetStringLibrary.Concat_StrStr` "Max X :" (`KismetStringLibrary.Conv_DoubleToString` _output_get_4)) true true (struct :`G` 0.66 :`B` 1.0 :`A` 1.0) 11.0)
      (goto _label))
    (:`Out 3`
      (bind _output_get_5 (set `self.MaxY` (`KismetMathLibrary.Abs` (+ (.y _origin) (.y _boxextent)))))
      (set `self.MaxArea_Y` _output_get_5)
      (`KismetSystemLibrary.PrintString` (`KismetStringLibrary.Concat_StrStr` "Max Y :" (`KismetStringLibrary.Conv_DoubleToString` _output_get_5)) true true (struct :`G` 0.66 :`B` 1.0 :`A` 1.0) 11.0)
      (goto _label))
    (:`Out 4`
      (`self.DrawGrid`)
      (set `self.StartNode` (`|GetArrayItem` (`self.NodeArray`)))
      (set `self.DestNode` (`|GetArrayItem` _nodearray (- (`KismetArrayLibrary.Array_Length` _nodearray) 1))))))

(event `self.ReceiveBeginPlay`
  (bind _returnvalue (`|CreateWidget` "/Game/Blueprint/UI/BP_AlgorithmUI.BP_AlgorithmUI_C"))
  (`UserWidget.AddToViewport` _returnvalue 0)
  (bind _output_get (set `self.FinderUI` _returnvalue))
  (add `Button.OnClicked` (`AlgorithmUI.Astar_button` _output_get) (`self.Astar_Delegate`))
  (add `Button.OnClicked` (`AlgorithmUI.Dijkstra_button` _output_get) (`self.Dijkstra_Delegate`))
  (add `Button.OnClicked` (`AlgorithmUI.BFS_button` _output_get) (`self.BFS_Delegate`))
  (`parent.ReceiveBeginPlay`)
  (bind _outactors (`GameplayStatics.GetAllActorsWithTag` "Plain"))
  (bind _output (`|GetArrayItem` _outactors))
  (set `self.Area` _output)
  (`KismetSystemLibrary.PrintString` (`KismetSystemLibrary.GetDisplayName` _output))
  (set `self.AreaBox` (`self.GetComponentByClass` (`self.Area`) "/Script/Engine.BoxComponent"))
  (goto _label))

(fn `UserConstructionScript`)