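; BP_Node_CrossLine is a graph node actor with a cost and connections, likely for pathfinding.
; BeginPlay assigns a random integer cost and labels the node with its name suffix and cost.
; SetNodeCunnection links it to other CrossLine nodes overlapping its collision sphere.
; OverlappedCheck flags "Wall" overlaps and lifts nodes on "Mount" actors to the bounds top, then steps them down until something overlaps again.
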(event `self.ReceiveBeginPlay`
  (bind _returnvalue (`KismetSystemLibrary.GetDisplayName` (`ActorComponent.GetOwner` (`self.Sphere`))))
  (set `self.CollisionMesh` (`self.Sphere Collision`))
  (`KismetSystemLibrary.LogString` _returnvalue)
  (`self.SetNodeCost` (`KismetMathLibrary.RandomIntegerInRange` 0 5))
  (`TextRenderComponent.K2_SetText` (`self.NodeText`) (`KismetTextLibrary.Conv_StringToText` (`KismetStringLibrary.Concat_StrStr` (`.RightS` (`KismetStringLibrary.Split` _returnvalue "BP_Node_CrossLine_")) " / " (`KismetStringLibrary.Conv_IntToString` (`KismetMathLibrary.Round` (`self.nodeCost`)))))))

(event `self.SetNodeCunnection`
  (`self.AddConnection` (`PrimitiveComponent.GetOverlappingActors` (`self.Sphere Collision`) "BP_Node_CrossLine_C")))

(fn `OverlappedCheck`
  (returns (Result :type Boolean))
  (bind (_returnvalue_x _returnvalue_y _returnvalue_z) (`KismetMathLibrary.BreakVector` (`self.K2_GetActorLocation`)))
  (bind _returnvalue (`self.GetTransform`))
  (bind _returnvalue_2 (`KismetArrayLibrary.Array_IsValidIndex` (`PrimitiveComponent.GetOverlappingActors` (`self.Sphere Collision`) null)))
  (for _array_element (`PrimitiveComponent.GetOverlappingActors` (`self.Sphere Collision`) null)
    (if (`self.ActorHasTag` _array_element "Wall")
      (set `self.overlapped` true)
      (break)
      (elif (`self.ActorHasTag` _array_element "Mount")
        (bind (_origin _boxextent) (`self.GetActorBounds` _array_element false false))
        (`self.K2_SetActorTransform` (`KismetMathLibrary.MakeTransform` (`KismetMathLibrary.MakeVector` (.x (.location _returnvalue)) (.y (.location _returnvalue)) (+ (.z _origin) (.z _boxextent))) (.rotation _returnvalue) (.scale _returnvalue)))
        (if (not _returnvalue_2)
          (while (not _returnvalue_2)
            (`self.K2_SetActorTransform` (`KismetMathLibrary.MakeTransform` (`KismetMathLibrary.MakeVector` (.x (.location _returnvalue)) (.y (.location _returnvalue)) (- _returnvalue_z 5.0)) (.rotation _returnvalue) (.scale _returnvalue))))
          (`KismetSystemLibrary.PrintString` "Set Position ")))))
  (return (`self.overlapped`)))

(fn `UserConstructionScript`)